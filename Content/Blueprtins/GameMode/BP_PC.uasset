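; BP_PC is a player controller that handles respawn requests and text chat for a multiplayer game.
; Server_Respawn passes the controller to BP_GM to respawn the player.
; Enter focuses the UMGChatting text box unless it already has keyboard focus.
; Server_SendMessage prefixes the sender's player name and relays the text to every BP_PC, whose Client_ReciveMessage updates that chat widget.
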(event `Server_Respawn`
  (bind _returnvalue (`GameplayStatics.GetGameMode`))
  (`/Engine/EditorBlueprintResources/StandardMacros.IsValid` _returnvalue
    (:`Is Valid`
      (bind _asbp_gm (cast `/Game/Blueprtins/GameMode/BP_GM` _returnvalue))
      (`/Game/Blueprtins/GameMode/BP_GM.Server_RespawnPlayer` _asbp_gm self))))

(event `Key|Enter`
  (params (Key :type "Key Structure"))
  (bind _editabletext (`/Game/Blueprtins/UMG/UMG_Chatting.EditableText` (`self.UMG_Chatting`)))
  (:`Pressed`
    (if (not (`Widget.HasKeyboardFocus` _editabletext))
      (`Widget.SetFocus` _editabletext))))

(event `Client_ReciveMessage`
  (params (`In Text` :type Text))
  (bind _umg_chatting (`self.UMG_Chatting`))
  (`/Engine/EditorBlueprintResources/StandardMacros.IsValid` _umg_chatting
    (:`Is Valid`
      (`/Game/Blueprtins/UMG/UMG_Chatting.UpdateChat` _umg_chatting `In Text`))))

(event `Server_SendMessage`
  (params (`In Text` :type Text))
  (bind _outactors (`GameplayStatics.GetAllActorsOfClass` "BP_PC_C"))
  (for _array_element _outactors
    (`self.Client_ReciveMessage` _array_element (`KismetTextLibrary.Conv_StringToText` (`KismetStringLibrary.Concat_StrStr` (`PlayerState.GetPlayerName` (`self.PlayerState`)) ":" (`KismetTextLibrary.Conv_TextToString` `In Text`))))))

(fn `UserConstructionScript`)